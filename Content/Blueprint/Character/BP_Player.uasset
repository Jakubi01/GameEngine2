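; BP_Player is the player character Blueprint that keeps the on-screen health and score readouts up to date.
; On BeginPlay it casts the player controller's HUD to BP_MainHUD, caches it, and binds to its health-changed and point-changed delegates.
; Each delegate handler formats the new value into a labelled string and writes it to the matching text block in the HUD's PlayerStatusWidget.
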(event `self.ReceiveBeginPlay`
  (bind _asbp_main_hud (cast `/Game/Blueprint/Widgets/BP_MainHUD` (`PlayerController.GetHUD` (`GameplayStatics.GetPlayerController` 0))))
  (set `self.BP Main HUD` _asbp_main_hud)
  (add `self.OnHealthChangedDelegate` (delegate `OnHealthChangedDelegate_이벤트`))
  (add `self.OnPointChangedDelegate` (delegate `OnPointChangedDelegate_이벤트`)))

(event `OnHealthChangedDelegate_이벤트` :!signature `self.OnHealthChangedDelegate`
  (params (health :type Integer))
  (`TextBlock.SetText` (`/Game/Blueprint/Widgets/WBP_PlayerStatus.PlayerHealth_Text` (`/Game/Blueprint/Widgets/BP_MainHUD.PlayerStatusWidget` (`self.BP Main HUD`))) (`|GenericToText` (`KismetStringLibrary.Concat_StrStr` "Health : " (`KismetStringLibrary.Conv_IntToString` health)))))

(event `OnPointChangedDelegate_이벤트` :!signature `self.OnPointChangedDelegate`
  (params (point :type Integer))
  (`TextBlock.SetText` (`/Game/Blueprint/Widgets/WBP_PlayerStatus.GamePoint_Text` (`/Game/Blueprint/Widgets/BP_MainHUD.PlayerStatusWidget` (`self.BP Main HUD`))) (`|GenericToText` (`KismetStringLibrary.Concat_StrStr` "Score : " (`KismetStringLibrary.Conv_IntToString` point)))))

(fn `UserConstructionScript`)