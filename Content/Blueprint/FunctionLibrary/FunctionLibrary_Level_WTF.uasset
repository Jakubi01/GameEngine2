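; Blueprint function library with a helper, SetLevelState, that sets the first player's cursor visibility and input mode.
; It shows or hides the mouse cursor on player controller 0, then switches between Game Only, Game and UI, or UI Only input.
; The Pause parameter has no effect because its SetGamePaused call is never executed.
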(fn `SetLevelState`
  (params (Pause :type Boolean) (CursorVisible :type Boolean) (InputMode :type "/Game/Blueprint/GameMode/EInputMode Enum" :default "NewEnumerator0"))
  (bind _returnvalue (`GameplayStatics.GetPlayerController` null))
  (set `PlayerController.bShowMouseCursor` (`local.CursorVisible`) (`GameplayStatics.GetPlayerController` null))
  (switch `/Game/Blueprint/GameMode/EInputMode` (`local.InputMode`)
    (:`NewEnumerator0`
      (`WidgetBlueprintLibrary.SetInputMode_GameOnly` _returnvalue))
    (:`NewEnumerator1`
      (`WidgetBlueprintLibrary.SetInputMode_GameAndUIEx` _returnvalue null))
    (:`NewEnumerator2`
      (`WidgetBlueprintLibrary.SetInputMode_UIOnlyEx` _returnvalue null))))