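; BP_DBM_GameMode is a game mode that handles the game-over sequence for a win or defeat.
; On BeginPlay it caches the main HUD and WTFPlayer character, then binds the game-over delegate.
; When that fires, it pauses the level, saves the player's points through the game instance's high-score setter and destroys enemies.
; After a short delay it shows the score and result text, then destroys the player.
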(event `self.ReceiveBeginPlay`
  (set `self.bGameOver` false)
  (`|ExecutionSequence`
    (:`then_0`
      (bind _asbp_main_hud (cast `/Game/Blueprint/Widgets/BP_MainHUD` (`PlayerController.GetHUD` (`GameplayStatics.GetPlayerController` 0))))
      (set `self.CachedMainHUD` _asbp_main_hud)
      (bind _aswtfplayer (cast `WTFPlayer` (`GameplayStatics.GetPlayerCharacter` 0)))
      (set `self.CachedPlayerCharacter` _aswtfplayer))
    (:`then_1`
      (add `self.OnGameOverDelegate` (delegate `OnGameOverDelegate_이벤트`)))))

(event `OnGameOverDelegate_이벤트` :!signature `self.OnGameOverDelegate`
  (params (state :type "EGameOverState Enum" :default "Defeat"))
  (bind (_aswtfgame_instance _bsuccess) (cast `WTFGameInstance` (`GameplayStatics.GetGameInstance`) :!pure true))
  (bind _gameoverwidget (`/Game/Blueprint/Widgets/BP_MainHUD.GameOverWidget` (`self.CachedMainHUD`)))
  (`|ExecutionSequence`
    (:`then_0`
      (set `self.bGameOver` true)
      (`/Game/Blueprint/FunctionLibrary/FunctionLibrary_Level_WTF.SetLevelState` true true "NewEnumerator2")
      (if _bsuccess
        (`WTFGameInstance.SetHighScore` _aswtfgame_instance (`WTFPlayer.GetPoint` (`self.CachedPlayerCharacter`)))))
    (:`then_1`
      (`WTFBlueprintFunctionLibrary.DestroyAllEnemyObject` (`self.CachedPlayerCharacter`))
      (`KismetSystemLibrary.Delay` 0.3)
      (`/Game/Blueprint/Widgets/WBP_GameOver.ShowScore` _gameoverwidget)
      (`/Game/Blueprint/Widgets/WBP_GameOver.SetWidgetVisible` _gameoverwidget "Visible")
      (switch `EGameOverState` state
        (:`Defeat`
          (`TextBlock.SetText` (`/Game/Blueprint/Widgets/WBP_GameOver.GameOverState_Text` (`/Game/Blueprint/Widgets/BP_MainHUD.GameOverWidget` (`self.CachedMainHUD`))) (`self.DefeatText`)))
        (:`Win`
          (`TextBlock.SetText` (`/Game/Blueprint/Widgets/WBP_GameOver.GameOverState_Text` (`/Game/Blueprint/Widgets/BP_MainHUD.GameOverWidget` (`self.CachedMainHUD`))) (`self.WinText`))))
      (`self.K2_DestroyActor` (`self.CachedPlayerCharacter`)))))

(fn `UserConstructionScript`)